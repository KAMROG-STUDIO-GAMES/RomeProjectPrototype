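; Actor component in the Districts folder that handles timed, resource-paid level upgrades for its owner.
; Starting an upgrade checks the next level's cost, takes it from global storage and runs a timer, which also supplies progress.
; Ending it increments the level and calls ApplyNewLevel, an empty hook.
; Availability is recomputed on upgrade start, end and storage changes, then broadcast to listeners.
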(event `self.ReceiveBeginPlay`
  (`parent.ReceiveBeginPlay`)
  (add `/Game/RomeProject/Districts/AC_Storage.OnResourceAmountChanged` (`.Component` (`/Game/RomeProject/Core/BPFL_Utilities.GetGlobalStorage`)) (delegate `OnResourceAmountChanged_Event_0`)))

(event `OnResourceAmountChanged_Event_0`
  (params (ResourceType :type "/Game/RomeProject/Core/E_Resources Enum" :default "NewEnumerator0") (OldValue :type "Float (double-precision)") (NewValue :type "Float (double-precision)"))
  (`self.UpdateUpgradeAvailability`))

(fn `ApplyNewLevel`
  (params (NewLevel :type Integer)))

(fn `CanBeUpgraded`
  (returns (Value :type Boolean))
  (return (and (< (`self.CurrentLevel`) (`self.MaxLevel`)) (not (`self.Upgrading`)))))

(fn `EndUpgrading`
  (bind _currentlevel (`self.CurrentLevel`))
  (`/Engine/EditorBlueprintResources/StandardMacros.IncrementInt` (`self.CurrentLevel`)
    (:`  `
      (set `self.Upgrading` false)
      (`KismetSystemLibrary.K2_ClearAndInvalidateTimerHandle` (`self.UpgradeTimer`))
      (`self.ApplyNewLevel` _currentlevel)
      (`KismetSystemLibrary.PrintString` (`KismetTextLibrary.Conv_TextToString` (`|FormatText` "Current {m} level is {n}" (`self.GetOwner`) _currentlevel)) true true (struct :`G` 1.0 :`B` 0.017425 :`A` 1.0))
      (`self.UpdateUpgradeAvailability`))))

(fn `Get Current Upgrade Cost`
  (returns (Resources :type "Array of /Game/RomeProject/Core/F_Resource Structure"))
  (return (`.Resources_15_F5AEF299403248B82FE39A96EA57571E` (break `/Game/RomeProject/Core/F_UpgradeCost` (`|GetArrayItem` (`self.Upgrades`) (+ (`self.CurrentLevel`) 1))))))

(fn `GetCurrentUpgradeTime`
  (returns (Time :type "Float (double-precision)"))
  (return (`.Time_12_73278C8A40BDC298CEA0D791BA78E979` (break `/Game/RomeProject/Core/F_UpgradeCost` (`|GetArrayItem` (`self.Upgrades`) (+ (`self.CurrentLevel`) 1))))))

(fn `GetUpgradeAvailability`
  (returns (UpgradeAvailable :type Boolean))
  (return (`self.UpgradeAvailable`)))

(fn `GetUpgradeProgress`
  (returns (NormalizedValue :type "Float (double-precision)"))
  (if (`self.Upgrading`)
    (return (/ (`KismetSystemLibrary.K2_GetTimerElapsedTimeHandle` (`self.UpgradeTimer`)) (`self.GetCurrentUpgradeTime`)))
    (else
      (return 0.0))))

(fn `StartUpgrading`
  (locals (UpgradeData :type "/Game/RomeProject/Core/F_UpgradeCost Structure"))
  (bind (_level _time _resources) (break `/Game/RomeProject/Core/F_UpgradeCost` (`local.UpgradeData`)))
  (set `local.UpgradeData` (`|GetArrayItem` (`self.Upgrades`) (+ (`self.CurrentLevel`) 1)))
  (bind _value (`/Game/RomeProject/Core/BPFL_Utilities.IsEnoughGlobalResources?` _resources))
  (if _value
    (bind _returnvalue (`KismetSystemLibrary.K2_SetTimerDelegate` (`|CreateDelegate` :!event `EndUpgrading`) _time))
    (set `self.UpgradeTimer` _returnvalue)
    (set `self.Upgrading` true)
    (`/Game/RomeProject/Districts/AC_Storage.TakeFromStorage` (`.Component` (`/Game/RomeProject/Core/BPFL_Utilities.GetGlobalStorage`)) _resources)
    (`self.UpdateUpgradeAvailability`)
    (`self.OnUpgradeStarted`)
    (else
      (`KismetSystemLibrary.PrintString` "Not enough resources to upgrade" true true (struct :`R` 1.0 :`G` 0.58537 :`A` 1.0)))))

(fn `UpdateUpgradeAvailability`
  (bind _value (`/Game/RomeProject/Core/BPFL_Utilities.IsEnoughGlobalResources?` (`.Resources_15_F5AEF299403248B82FE39A96EA57571E` (break `/Game/RomeProject/Core/F_UpgradeCost` (`|GetArrayItem` (`self.Upgrades`) (+ (`self.CurrentLevel`) 1))))))
  (bind _output_get (set `self.UpgradeAvailable` (and (< (`self.CurrentLevel`) (`self.MaxLevel`)) (not (`self.Upgrading`)) _value)))
  (`self.OnUpgradeAvailabilityChanged` _output_get))