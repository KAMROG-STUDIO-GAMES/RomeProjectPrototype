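; AC_Storage is an actor component that holds resource amounts and per-resource capacities, with batch add, take and sufficiency checks.
; Amount changes go through SetResourceAmount, which clamps to capacity, prints overflow or invalid-resource warnings and broadcasts OnResourceAmountChanged on writes.
; Both arrays are indexed by resource enum; zero capacity marks unaccepted resources, which bulk capacity edits skip.
; Placeholder EmptyStorage moves contents into the first BP_StorageDistrict found.
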(event `self.ReceiveBeginPlay`
  (set `self.Capacity` (`self.InitialCapacity`)))

(event `self.ReceiveTick`
  (params (DeltaSeconds :type "Float (single-precision)")))

(fn `AddResourceAmount`
  (params (ResourceType :type "/Game/RomeProject/Core/E_Resources Enum" :default "NewEnumerator0") (Amount :type "Float (double-precision)"))
  (`self.SetResourceAmount` ResourceType (+ Amount (`self.GetResourceAmount` ResourceType))))

(fn `AddResourceCapacity`
  (params (Resource :type "/Game/RomeProject/Core/E_Resources Enum" :default "NewEnumerator0") (Amount :type "Float (double-precision)"))
  (`self.SetResourceCapacity` Resource (+ Amount (`self.GetResourceCapacity` Resource))))

(fn `AddToStorage`
  (params (Resources :type "Array of /Game/RomeProject/Core/F_Resource Structure"))
  (locals (MaxCapacity :type "Float (double-precision)") (AmountToAdd :type "Float (double-precision)") (ResourceType :type "/Game/RomeProject/Core/E_Resources Enum"))
  (for _array_element Resources
    (bind (_resource _amount) (break `/Game/RomeProject/Core/F_Resource` _array_element))
    (`self.AddResourceAmount` _resource _amount)))

(fn `EmptyStorage`
  (bind _storedresources (`self.GetStoredResources`))
  ;[1 1 1] Change this placeholder
  (bind _outactors (`GameplayStatics.GetAllActorsOfClass` "/Game/RomeProject/Districts/BP_StorageDistrict.BP_StorageDistrict_C"))
  (`self.AddToStorage` (`Actor.GetComponentByClass` (`|GetArrayItem` _outactors) "AC_Storage_C") _storedresources)
  (`self.TakeFromStorage` _storedresources))

(fn `GetCapacity`
  (returns (Capacity :type "Array of /Game/RomeProject/Core/F_Resource Structure"))
  (return (`self.Capacity`)))

(fn `GetResourceAmount`
  (params (ResourceType :type "/Game/RomeProject/Core/E_Resources Enum" :default "NewEnumerator0"))
  (returns (Amount :type "Float (double-precision)"))
  (return (`.Amount_5_D9C63C9D4830F6146E31A0A364966600` (break `/Game/RomeProject/Core/F_Resource` (`|GetArrayItem` (`self.StoredResources`) (`KismetMathLibrary.Conv_ByteToInt` ResourceType))))))

(fn `GetResourceCapacity`
  (params (ResourceType :type "/Game/RomeProject/Core/E_Resources Enum" :default "NewEnumerator0"))
  (returns (Amount :type "Float (double-precision)"))
  (return (`.Amount_5_D9C63C9D4830F6146E31A0A364966600` (break `/Game/RomeProject/Core/F_Resource` (`|GetArrayItem` (`self.Capacity`) (`KismetMathLibrary.Conv_ByteToInt` ResourceType))))))

(fn `GetStoredResources`
  (returns (StoredResources :type "Array of /Game/RomeProject/Core/F_Resource Structure"))
  (return (`self.StoredResources`)))

(fn `IncreaseAllValidCapacities`
  (params (Value :type "Float (double-precision)"))
  (for _array_element (`self.Capacity`)
    (bind (_resource _amount) (break `/Game/RomeProject/Core/F_Resource` _array_element))
    (if (!= _amount 0.0)
      (`self.AddResourceCapacity` _resource (`local.Value`)))))

(fn `IsEnoughtResources?`
  (params (Resources :type "Array of /Game/RomeProject/Core/F_Resource Structure"))
  (returns (Result :type Boolean))
  (for _array_element Resources
    (bind (_resource _amount) (break `/Game/RomeProject/Core/F_Resource` _array_element))
    (if (< (`self.GetResourceAmount` _resource) _amount)
      (return false)))
  (return true))

(fn `MultiplyAllValidCapacities`
  (params (Value :type "Float (double-precision)"))
  (for _array_element (`self.Capacity`)
    (bind (_resource _amount) (break `/Game/RomeProject/Core/F_Resource` _array_element))
    (if (!= _amount 0.0)
      (`self.SetResourceCapacity` _resource (* _amount (`local.Value`))))))

(fn `SetAllValidCapacities`
  (params (Value :type "Float (double-precision)"))
  (for _array_element (`self.Capacity`)
    (bind (_resource _amount) (break `/Game/RomeProject/Core/F_Resource` _array_element))
    (if (!= _amount 0.0)
      (`self.SetResourceCapacity` _resource (`local.Value`)))))

(fn `SetCapacity`
  (params (Capacity :type "Array of /Game/RomeProject/Core/F_Resource Structure"))
  (set `self.Capacity` Capacity))

(fn `SetResourceAmount`
  (params (ResourceType :type "/Game/RomeProject/Core/E_Resources Enum" :default "NewEnumerator0") (Amount :type "Float (double-precision)"))
  (bind _resourcetype (`local.ResourceType`))
  (bind _amount (`self.GetResourceCapacity` (`local.ResourceType`)))
  (bind _returnvalue (`KismetMathLibrary.FClamp` (`local.Amount`) 0.0 (`self.GetResourceCapacity` (`local.ResourceType`))))
  (if (> Amount _amount)
    (`KismetSystemLibrary.PrintString` (`KismetTextLibrary.Conv_TextToString` (`|FormatText` "{x}: storage is full!" (`|GetEnumeratorNameAsString` (`local.ResourceType`)))) true true (struct :`R` 1.0 :`G` 0.496819 :`A` 1.0))
    (`|VariableSetRef` (`|GetArrayItem` (`self.StoredResources`) (`KismetMathLibrary.Conv_ByteToInt` (`local.ResourceType`))) (make `/Game/RomeProject/Core/F_Resource` (`local.ResourceType`) _returnvalue) :!label _label)
    (`self.OnResourceAmountChanged` _resourcetype (`self.GetResourceAmount` _resourcetype) _returnvalue)
    (elif (!= _amount 0.0)
      (goto _label)
      (elif (!= (`local.Amount`) 0.0)
        (`KismetSystemLibrary.PrintString` (`KismetTextLibrary.Conv_TextToString` (`|FormatText` "{x} Incorrect resource added to storage. Resource deleted " (`KismetTextLibrary.Conv_StringToText` (`|GetEnumeratorNameAsString` (`local.ResourceType`))))) true true (struct :`R` 1.0 :`G` 0.011039 :`A` 1.0) 5.0)))))

(fn `SetResourceCapacity`
  (params (Resource :type "/Game/RomeProject/Core/E_Resources Enum" :default "NewEnumerator0") (Amount :type "Float (double-precision)"))
  (`|VariableSetRef` (`|GetArrayItem` (`self.Capacity`) (`KismetMathLibrary.Conv_ByteToInt` Resource)) (make `/Game/RomeProject/Core/F_Resource` Resource (`KismetMathLibrary.FMax` Amount))))

(fn `TakeFromStorage`
  (params (Resources :type "Array of /Game/RomeProject/Core/F_Resource Structure"))
  (locals (ResourceType :type "/Game/RomeProject/Core/E_Resources Enum") (Amount :type "Float (double-precision)"))
  (for _array_element Resources
    (bind (_resource _amount) (break `/Game/RomeProject/Core/F_Resource` _array_element))
    (`self.AddResourceAmount` _resource (* -1 _amount))))