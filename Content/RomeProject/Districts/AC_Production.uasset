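; Actor component for districts that periodically produces a resource into the owner's AC_Storage component.
; On BeginPlay it copies the initial tick time and amount, then starts a looping timer.
; ProductionTick adds the amount times a multiplier of the configured resource type to storage, if present.
; Setters re-arm the timer for tick changes or fire change dispatchers for amount and multiplier; a getter exposes its widget class.
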(event `self.ReceiveBeginPlay`
  (set `self.Tick` (`self.InitialTickTime`))
  (set `self.ProductionAmount` (`self.InitialProductionAmount`))
  (`self.SetupTimer`))

(fn `GetProductionAmount`
  (returns (ProductionAmount :type "Float (double-precision)"))
  (return (`self.ProductionAmount`)))

(fn `GetProductionMultiplier`
  (returns (ProductionMultiplier :type "Float (double-precision)"))
  (return (`self.ProductionMultiplier`)))

(fn `GetProductionTick`
  (returns (Tick :type "Float (double-precision)"))
  (return (`self.Tick`)))

(fn `GetWidgetClass`
  (returns (Widget :type "/Game/RomeProject/Widgets/WBP_ComponentWidgetBase Class Reference"))
  (return (`self.WidgetClass`)))

(fn `ProductionTick`
  (locals (StorageComp :type "/Game/RomeProject/Districts/AC_Storage Object Reference"))
  (bind _output_get (set `local.StorageComp` (`Actor.GetComponentByClass` (`self.GetOwner`) "/Game/RomeProject/Districts/AC_Storage.AC_Storage_C")))
  (`/Engine/EditorBlueprintResources/StandardMacros.IsValid` _output_get
    (:`Is Valid`
      (`/Game/RomeProject/Districts/AC_Storage.AddToStorage` (`local.StorageComp`) (`|MakeArray` (make `/Game/RomeProject/Core/F_Resource` (`self.ResourceType`) (* (`self.ProductionAmount`) (`self.ProductionMultiplier`))) :!type "/Game/RomeProject/Core/F_Resource Structure")))))

(fn `SetProductionAmount`
  (params (ProductionAmount :type "Float (double-precision)"))
  (bind _output_get (set `self.ProductionAmount` ProductionAmount))
  (`self.OnProductionAmountChanged` _output_get))

(fn `SetProductionMultiplier`
  (params (ProductionMultiplier :type "Float (double-precision)"))
  (bind _output_get (set `self.ProductionMultiplier` ProductionMultiplier))
  (`self.OnProductionMultiplierChanged` _output_get))

(fn `SetProductionTick`
  (params (Tick :type "Float (double-precision)"))
  (set `self.Tick` Tick)
  (`self.SetupTimer`))

(fn `SetupTimer`
  (bind _returnvalue (`KismetSystemLibrary.K2_SetTimerDelegate` (`|CreateDelegate` :!event `ProductionTick`) (`self.Tick`) true))
  (set `self.ProductionTimer` _returnvalue))