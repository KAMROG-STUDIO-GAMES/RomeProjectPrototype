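; AC_Gathering is an actor component that spawns a gathering interaction when its owner's stored resources reach trigger amounts.
; On BeginPlay it binds to the owner's AC_Storage amount-change event, printing an error if none exists.
; Matching triggers spawn a BP_Gathering beside the owner, whose completion clears InteractionActive and empties storage.
; InteractionActive guards spawning, though these graphs never set it true.
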(event `self.ReceiveBeginPlay`
  (bind _returnvalue (`Actor.GetComponentByClass` (`self.GetOwner`) "/Game/RomeProject/Districts/AC_Storage.AC_Storage_C"))
  (`/Engine/EditorBlueprintResources/StandardMacros.IsValid` _returnvalue
    (:`Is Valid`
      (bind _output_get (set `self.StorageComp` _returnvalue))
      (add `/Game/RomeProject/Districts/AC_Storage.OnResourceAmountChanged` _output_get (`|CreateDelegate` :!event `HandleTriggers`)))
    (:`Is Not Valid`
      (`KismetSystemLibrary.PrintString` "InitError" true true (struct :`R` 1.0 :`B` 0.072882 :`A` 1.0)))))

(fn `CreateInteraction`
  (if (not (`self.InteractionActive`))
    (bind _returnvalue (`|SpawnActorFromClass` "/Game/RomeProject/Districts/BP_Gathering.BP_Gathering_C" (`KismetMathLibrary.MakeTransform` (+ (`Actor.K2_GetActorLocation` (`self.GetOwner`)) (0.0 20.0 20.0))) "Undefined" "OverrideRootScale" null null))
    (add `/Game/RomeProject/Districts/BP_Gathering.OnGatheringComplete` _returnvalue (`|CreateDelegate` :!event `HandleGatheringComplete`))))

(fn `HandleGatheringComplete`
  (set `self.InteractionActive` false)
  (`/Game/RomeProject/Districts/AC_Storage.EmptyStorage` (`self.StorageComp`)))

(fn `HandleTriggers`
  (params (ResourceType :type "/Game/RomeProject/Core/E_Resources Enum" :default "NewEnumerator0") (OldValue :type "Float (double-precision)") (NewValue :type "Float (double-precision)"))
  (for _array_element (`self.Triggers`)
    (bind (_resource _amount) (break `/Game/RomeProject/Core/F_Resource` _array_element))
    (if (and (== _resource (`local.ResourceType`)) (>= (`local.NewValue`) _amount))
      (if (not (`self.InteractionActive`))
        (`self.CreateInteraction`)))))