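; Actor component that opens a configurable UI widget when its owning actor is clicked or touched, in the RomeProject districts.
; On BeginPlay it binds to the owner's click and touch-begin events, both of which call HandleInteraction.
; HandleInteraction creates the widget, passes it the owner as source and blocks further opens until the widget's close request.
; WidgetClosed removes the widget and re-enables opening.
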(event `self.ReceiveBeginPlay`
  (add `Actor.OnClicked` (`self.GetOwner`) (`|CreateDelegate` :!event `EventOwnerClicked`))
  (add `Actor.OnInputTouchBegin` (`self.GetOwner`) (`|CreateDelegate` :!event `EventOwnerTouch`)))

(event `EventOwnerTouch`
  (params (FingerIndex :type "ETouchIndex Enum" :default "Touch1") (TouchedActor :type "Actor Object Reference"))
  (`self.HandleInteraction` :!label _label))

(event `EventOwnerClicked`
  (params (TouchedActor :type "Actor Object Reference") (ButtonPressed :type "Key Structure" :default "None"))
  (goto _label))

(fn `HandleInteraction`
  (if (and (`self.CanOpenWidget`) (`KismetSystemLibrary.IsValidClass` (`self.WidgetToOpen`)))
    (bind _returnvalue (`|CreateWidget` (`self.WidgetToOpen`)))
    (bind _output_get (set `self.Widget` _returnvalue))
    (`UserWidget.AddToViewport` _output_get 0)
    (set `self.CanOpenWidget` false)
    (message `/Game/RomeProject/Widgets/BPI_WidgetInitialization.InitializeSourceRef` (`self.Widget`) (`self.GetOwner`))
    (add `/Game/RomeProject/Widgets/WBP_Base.CloseRequest` (`self.Widget`) (`|CreateDelegate` :!event `WidgetClosed`))))

(fn `WidgetClosed`
  (`Widget.RemoveFromParent` (`self.Widget`))
  (set `self.CanOpenWidget` true)
  (set `self.Widget` null))