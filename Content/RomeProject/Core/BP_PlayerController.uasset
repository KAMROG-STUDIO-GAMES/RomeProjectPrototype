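; Player controller for RomeProject that lets the player speed up or slow down game time.
; The SpeedUp and SlowDown input actions double or halve a GameSpeed variable, with no limits applied.
; Each press passes the new value to the Cheat Manager's Slomo command, so time scaling depends on a cheat manager rather than setting global time dilation directly.
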(event `self.ReceiveBeginPlay`)

(event `InputAction|SpeedUp`
  (params (Key :type "Key Structure"))
  (:`Pressed`
    (bind _output_get (set `self.GameSpeed` (* (`self.GameSpeed`) 2.0)))
    (`CheatManager.Slomo` (`self.CheatManager`) _output_get)))

(event `InputAction|SlowDown`
  (params (Key :type "Key Structure"))
  (:`Pressed`
    (bind _output_get (set `self.GameSpeed` (/ (`self.GameSpeed`) 2.0)))
    (`CheatManager.Slomo` (`self.CheatManager`) _output_get)))

(fn `UserConstructionScript`)